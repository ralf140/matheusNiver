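; Dado actor that travels once along the spline of a referenced TrackR actor, then destroys itself.
; On BeginPlay, the MoveDado timeline drives a lerp from zero to the spline length, setting location and rotation at that distance each update.
; It samples the spline in local space and adds only the track actor's location, so the track's rotation and scale are not applied.
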(event `self.ReceiveBeginPlay`
  (bind _trackr (`self.trackR`))
  (bind _spline (`/Game/Blueprints/trackBp.Spline` _trackr))
  (bind (_direction _newtrack_0) (`Timeline|MoveDado`)
    (:`Update`
      (bind _returnvalue (`KismetMathLibrary.Lerp` 0.0 (`SplineComponent.GetSplineLength` _spline) _newtrack_0))
      (`self.K2_SetActorLocationAndRotation` (+ (`SplineComponent.GetLocationAtDistanceAlongSpline` _spline _returnvalue "Local") (`self.K2_GetActorLocation` _trackr)) (`SplineComponent.GetRotationAtDistanceAlongSpline` _spline _returnvalue "Local")))
    (:`Finished`
      (`self.K2_DestroyActor`))))

(fn `UserConstructionScript`)