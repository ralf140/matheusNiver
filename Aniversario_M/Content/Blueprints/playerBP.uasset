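; Player Blueprint for mouse-driven placement of MatheusBP actors on grid tiles, with a TorresMenu widget and visible cursor created at BeginPlay.
; While the SumonBo flag is set, a left click deprojects the cursor and line-traces on Visibility.
; A hit on a GridBp spawns MatheusBP at that actor's location and leaves the flag on.
; Any other result clears SumonBo, which nothing in this Blueprint sets to true.
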(event `Key|LeftMouseButton`
  (params (Key :type "Key Structure"))
  (bind (_worldlocation _worlddirection) (`PlayerController.DeprojectMousePositionToWorld` (`GameplayStatics.GetPlayerController` 0)))
  (:`Pressed`
    (if (`self.sumonBo`)
      (bind _outhit (`KismetSystemLibrary.LineTraceSingle` _worldlocation (+ _worldlocation (* _worlddirection (`self.NewVar`))) "TraceTypeQuery1"))
      (bind _asgrid_bp (cast `/Game/Blueprints/GridBp` (`.HitActor` (`GameplayStatics.BreakHitResult` _outhit)))
        (:`then`
          (`KismetSystemLibrary.PrintString` "nice")
          (`|SpawnActorFromClass` "/Game/Blueprints/matheusBP.matheusBP_C" (`KismetMathLibrary.MakeTransform` (`self.K2_GetActorLocation` _asgrid_bp)) "Undefined" "OverrideRootScale" null null))
        (:`CastFailed`
          (set `self.sumonBo` false)
          (`KismetSystemLibrary.PrintString` "not"))))))

(event `self.ReceiveBeginPlay`
  (bind _returnvalue (`GameplayStatics.GetPlayerController` 0))
  (set `PlayerController.bShowMouseCursor` true _returnvalue)
  (bind _returnvalue_2 (`|CreateWidget` "/Game/Blueprints/torresMenu.torresMenu_C" _returnvalue))
  (`UserWidget.AddToViewport` _returnvalue_2 0))

(fn `UserConstructionScript`)